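; AI controller for a Red Light, Green Light game that links its pawn to the nearest BP_GreenLightRedLightLine actor.
; SetupGreenLightRedLightLine scans all line actors, keeps the one closest to the controlled pawn, and writes it to the Blackboard as "Doll" with its location as "Pos".
; BeginPlay, Tick and the construction script are empty, and nothing in this graph calls the setup function.
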(event EventBeginPlay)

(event EventTick
  (params (DeltaSeconds :type Float%20%28single-precision%29)))

(fn ConstructionScript)

(fn SetupGreenLightRedLightLine
  (bind _returnvalue (Pawn|GetControlledPawn))
  (bind _blackboard (Variables|Default|GetBlackboard))
  (bind _returnvalue_2 (Transformation|GetActorLocation _returnvalue))
  (bind _outactors (Actor|GetAllActorsOfClass "/Game/Blueprints/BP_GreenLightRedLightLine.BP_GreenLightRedLightLine_C"))
  (Variables|Default|SetGreenLightRedLightLine (Utilities|Array|Get(acopy) _outactors))
  (for _array_element _outactors
    (Utilities|IsValid _returnvalue
      (:Is%20Valid
        (if (< (Math|Vector|VectorLength (- (Transformation|GetActorLocation _array_element) _returnvalue_2)) (Math|Vector|VectorLength (- _returnvalue_2 (Transformation|GetActorLocation (Variables|Default|GetGreenLightRedLightLine)))))
          (Variables|Default|SetGreenLightRedLightLine _array_element)))))
  (AI|Components|Blackboard|SetValueasObject _blackboard (Utilities|Name|MakeLiteralName "Doll") (Variables|Default|GetGreenLightRedLightLine))
  (AI|Components|Blackboard|SetValueasVector _blackboard (Utilities|Name|MakeLiteralName "Pos") (Transformation|GetActorLocation (Variables|Default|GetGreenLightRedLightLine))))